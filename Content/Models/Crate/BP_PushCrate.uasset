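; BP_PushCrate is a crate actor that limits its own vertical movement.
; BeginPlay records the starting height as the minimum and a point slightly above it as the maximum, then Tick resets the location every frame with Z clamped to that band, leaving X and Y free.
; An unconnected branch meant to play SFX while the crate has velocity, and stop it otherwise, never runs.
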(event EventBeginPlay
  (bind _self self)
  (bind _returnvalue (Transformation|GetActorLocation _self))
  (bind _z (Math|Vector|BreakVector _returnvalue))
  (Variables|Default|SetminZ _z)
  (Variables|Default|SetmaxZ (+ _z 3.0)))

(event Collision|EventActorBeginOverlap
  (params (OtherActor :type Actor%20Object%20Reference)))

(event EventTick
  (params (DeltaSeconds :type Float%20%28single-precision%29))
  (bind _returnvalue (Transformation|GetActorLocation))
  (bind (_x _y _z) (Math|Vector|BreakVector _returnvalue))
  (Utilities|FlowControl|Sequence
    (:then_0
      (Transformation|SetActorLocation (Math|Vector|MakeVector _x _y (Math|Float|Clamp(Float) _z (Variables|Default|GetminZ) (Variables|Default|GetmaxZ))) false false))))

(fn ConstructionScript)