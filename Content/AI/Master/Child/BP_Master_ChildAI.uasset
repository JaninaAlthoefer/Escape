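; BP_Master_ChildAI is a master Blueprint for child AI that exposes behavior state and writes it to the Blackboard.
; Getters and a setter cover risk-taking, follow target and Area 3 trigger state, with risk-taking at or above a fixed threshold setting the runner key.
; Other functions raise the Free and Area 3 trigger Blackboard flags.
; The event graph and construction script are empty, leaving these functions to be called externally.
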(event EventBeginPlay)

(event Collision|EventActorBeginOverlap
  (params (OtherActor :type Actor%20Object%20Reference)))

(event EventTick
  (params (DeltaSeconds :type Float%20%28single-precision%29)))

(fn ConstructionScript)

(fn CFGetRisktaking
  (return (Variables|Default|Getrisktaking)))

(fn CFGetTargettoFollow
  (return (Variables|Default|GettargetToFollow)))

(fn CFGetIsTriggered
  (return (Variables|Default|GetisArea3Triggered)))

(fn CFSetRisktaking
  (params (value :type Float%20%28single-precision%29))
  (Variables|Default|Setrisktaking value))

(fn CFSetRunnerBlackboard
  (bind _risktaking (CallFunction|CFGetRisktaking))
  (AI|Components|Blackboard|SetValueasBool (AI|GetBlackboard self) (LocalVariables|GetRunnerName) (>= _risktaking 5e+01))
  (return))

(fn CFSetFree
  (AI|Components|Blackboard|SetValueasBool (AI|GetBlackboard self) (Variables|Default|GetFree) true))

(fn CFSetArea3TriggerActive
  (AI|Components|Blackboard|SetValueasBool (AI|GetBlackboard self) (Variables|Default|GetArea3Trigger) true))