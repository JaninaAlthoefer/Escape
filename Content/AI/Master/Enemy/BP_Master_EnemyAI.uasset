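; Master enemy AI character that perceives the player and relays what it senses to its Ctrl_Master_EnemyAI controller's blackboard.
; Sight or capsule overlap sets the target, while losing sight records the player's location and any heard noise as a point of interest.
; Tick pushes compassion once and waypoints on task updates, and raises or lowers the gun using seen-rate thresholds with hysteresis.
; Construction attaches a gun mesh, and helper functions handle aggro speech and externally reported noises.
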(event OnPerceptionUpdated(AIPerception)
  (params (UpdatedActors :type Array%20of%20Actor%20Object%20References))
  (bind _aiperception (Variables|Default|GetAIPerception))
  ;[1 1 1] AI Perception Implementation
  (if (Utilities|Array|ContainsItem UpdatedActors (Variables|Default|GetPlayerCharacter))
    (if (Utilities|Array|ContainsItem (Class|AIPerceptionComponent|GetPerceivedActors _aiperception "/Script/AIModule.AISense_Sight") (Variables|Default|GetPlayerCharacter))
      (Default|CFUpdateBlackBoardObject (Variables|Default|GetAIController) (Variables|Default|GetTargetCharacter) (Variables|Default|GetPlayerCharacter))
      (if (not (Variables|Default|GetwillIgnore))
        (Class|SophisticatedAIEnemy|SetIsSeen true))
      (else
        (Default|CFUpdateBlackBoardObject (Variables|Default|GetAIController) (Variables|Default|GetTargetCharacter))
        (Class|SophisticatedAIEnemy|SetIsSeen false)
        (Default|CFUpdateBlackBoardBoolean (Variables|Default|GetAIController) "newSighting" true)
        (Utilities|FlowControl|Sequence
          (:then_0
            (Default|CFUpdateBlackBoardVector (Variables|Default|GetAIController) "TargetLocation" (Transformation|GetActorLocation (Game|GetPlayerCharacter 0))))
          (:then_1
            (if (Utilities|Array|ContainsItem (Class|AIPerceptionComponent|GetPerceivedActors _aiperception "/Script/AIModule.AISense_Hearing") (Variables|Default|GetPlayerCharacter))
              (bind _asside_scroller_character (Utilities|Casting|CastToSideScrollerCharacter (Variables|Default|GetPlayerCharacter)))
              (Default|CFUpdateBlackBoardVector (Variables|Default|GetAIController) "POI" (Variables|/Game/SideScrollerCPP/Blueprints/SideScrollerCharacter.SideScrollerCharacter_C|GetNoiseHeardLocation _asside_scroller_character))
              (Development|PrintString "heard noise"))))))))

(event OnComponentBeginOverlap(CapsuleComponent)
  (params (OverlappedComponent :type Primitive%20Component%20Object%20Reference) (OtherActor :type Actor%20Object%20Reference) (OtherComp :type Primitive%20Component%20Object%20Reference) (OtherBodyIndex :type Integer) (bFromSweep :type Boolean) (SweepResult :type Hit%20Result%20Structure%20%28by%20ref%29))
  ;[1 1 1] Touch Event Mock Up
  (if (== OtherActor (Variables|Default|GetPlayerCharacter))
    ;[1 1 1] AI Perception Implementation
    (Default|CFUpdateBlackBoardObject (Variables|Default|GetAIController) (Variables|Default|GetTargetCharacter) (Variables|Default|GetPlayerCharacter))
    (if (not (Variables|Default|GetwillIgnore))
      (Class|SophisticatedAIEnemy|SetIsSeen true))))

(event EventBeginPlay
  ;[1 1 1] AI Setup
  (Variables|Default|SetPlayerCharacter (Game|GetPlayerCharacter 0))
  (bind _returnvalue (AI|GetAIController self))
  (bind _asctrl_master_enemy_ai (Utilities|Casting|CastToCtrl_Master_EnemyAI _returnvalue))
  (Variables|Default|SetAIController _asctrl_master_enemy_ai)
  (Default|CFUpdateBlackBoardVector (Variables|Default|GetAIController) "POI" "0, 0, 0")
  (Default|CFUpdateBlackBoardVector (Variables|Default|GetAIController) "TargetLocation" "0, 0, 0")
  (Default|CFUpdateBlackBoardBoolean (Variables|Default|GetAIController) "newSighting" true)
  (bind _outactors (Actor|GetAllActorsOfClass "/Game/AI/Master/Child/BP_Master_ChildAI.BP_Master_ChildAI_C"))
  (Variables|Default|SetChildrenArray _outactors))

(event EventTick
  (params (DeltaSeconds :type Float%20%28single-precision%29))
  (Utilities|FlowControl|Sequence
    (:then_0
      ;[1 1 1] Set Compassion
      (if (Variables|Default|GetfirstTick)
        (bind _returnvalue (Class|SophisticatedAIEnemy|IsCompassionate self))
        (Default|CFUpdateBlackBoardBoolean (Variables|Default|GetAIController) "IsCompassionate" _returnvalue)
        (Variables|Default|SetfirstTick false)))
    (:then_1
      ;[1 1 1] Was Task Updated?
      (if (Variables|Default|GettaskIsUpdated)
        (bind _returnvalue_2 (Class|SophisticatedAIEnemy|GetWaypoint 1))
        (Default|CFUpdateBlackBoardVector (Variables|Default|GetAIController) (Variables|Default|GetWaypoint1) _returnvalue_2)
        (bind _returnvalue_3 (Class|SophisticatedAIEnemy|GetWaypoint 2))
        (Default|CFUpdateBlackBoardVector (Variables|Default|GetAIController) (Variables|Default|GetWaypoint2) _returnvalue_3)
        (bind _returnvalue_4 (Class|SophisticatedAIEnemy|GetWaypoint 3))
        (Default|CFUpdateBlackBoardVector (Variables|Default|GetAIController) (Variables|Default|GetWaypoint3) _returnvalue_4)
        (Variables|Default|SettaskIsUpdated false)))
    (:then_2
      ;[1 1 1] Animation Setup
      (bind _seenrate (CallFunction|CFGetSeenRate))
      (if (> _seenrate 7e+01)
        (Variables|Default|SetRaisedGun? true)
        (elif (not (> _seenrate 5e+01))
          (Variables|Default|SetRaisedGun? false))))))

(fn ConstructionScript
  (bind _returnvalue (AddComponent|AddStaticMeshComponent true))
  (Transformation|AttachComponentToComponent _returnvalue (Variables|Character|GetMesh) "GunSocket" "KeepRelative" "KeepRelative" "KeepRelative" true))

(fn CFGetSeenRate
  (return (Variables|Default|GetseenRate)))

(fn CFSetIsSeen
  (params (bool :type Boolean))
  (Class|SophisticatedAIEnemy|SetIsSeen bool)
  (return))

(fn CFWasAggroed
  (Audio|PlaySoundatLocation "/Game/Audio/Dialogue/EnemySpeechCue.EnemySpeechCue" (Transformation|GetWorldLocation (Variables|Character|GetMesh)) "0, 0, 0" 0.7))

(fn CFSetPOINonPC
  (params (HeardAt :type Vector))
  (Default|CFUpdateBlackBoardVector (Variables|Default|GetAIController) "POI" HeardAt))